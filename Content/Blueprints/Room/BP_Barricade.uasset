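; BP_Barricade is a room prop made of five wooden plank pieces.
; Its construction script clears and refills the Planks array with those planks in a fixed, non-sequential order.
; The event graph holds only disabled placeholder events, so the Blueprint's own graphs add no runtime behavior.
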(fn `UserConstructionScript`
  (locals (NewLocalVar :type "StaticMeshComponent Object Reference"))
  (bind _planks (`self.Planks`))
  (`KismetArrayLibrary.Array_Clear` _planks)
  (`KismetArrayLibrary.Array_Add` _planks (`self.SM_Prop_WoodPlank_05`))
  (`KismetArrayLibrary.Array_Add` _planks (`self.SM_Prop_WoodPlank_04`))
  (`KismetArrayLibrary.Array_Add` _planks (`self.SM_Prop_WoodPlank_01`))
  (`KismetArrayLibrary.Array_Add` _planks (`self.SM_Prop_WoodPlank_03`))
  (`KismetArrayLibrary.Array_Add` _planks (`self.SM_Prop_WoodPlank_02`)))