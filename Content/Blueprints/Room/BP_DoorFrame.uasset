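; BP_DoorFrame is a room door frame actor that hides its decal and two rect lights when a door-opened event fires.
; The construction script stores the child actor of its BPDoor component as DoorPart.
; On BeginPlay it binds to OnDoorOpenedEvent, whose handler switches the visibility off, with no logic here to restore it.
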(event `self.ReceiveBeginPlay`
  (add `self.OnDoorOpenedEvent` (delegate `OnDoorOpenedEvent_Event`)))

(event `OnDoorOpenedEvent_Event`
  (`SceneComponent.SetVisibility` (`self.Decal`) false false)
  (`SceneComponent.SetVisibility` (`self.RectLight`) false false)
  (`SceneComponent.SetVisibility` (`self.RectLight1`) false false))

(fn `UserConstructionScript`
  (set `self.DoorPart` (`ChildActorComponent.ChildActor` (`self.BP_Door`))))