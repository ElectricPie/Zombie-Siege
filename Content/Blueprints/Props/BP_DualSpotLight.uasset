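; Dual spotlight prop whose left and right lamps, each a spot light and point light pair, can flicker independently at random intervals.
; When flickering is enabled, Tick compares game time against each side's random interval and starts a fast looping timer.
; The timer toggles that side's visibility for a random even count, then clears itself, toggles the lights back on and picks a new interval.
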(event `self.ReceiveBeginPlay`
  (bind _leftlights (`self.LeftLights`))
  (bind _rightlights (`self.RightLights`))
  (`KismetArrayLibrary.Array_Add` _rightlights (`self.SpotLightRight`))
  (`KismetArrayLibrary.Array_Add` _rightlights (`self.PointLightRight`))
  (`KismetArrayLibrary.Array_Add` _leftlights (`self.SpotLightLeft`))
  (`KismetArrayLibrary.Array_Add` _leftlights (`self.PointLightLeft`))
  (set `self.FlickerLeftInterval` (`self.Get Random Interval Time`))
  (set `self.FlickerRightInterval` (`self.Get Random Interval Time`)))

(event `self.ReceiveTick`
  (params (DeltaSeconds :type "Float (single-precision)"))
  (if (`self.LightCanFlicker`)
    (`|ExecutionSequence`
      (:`then_0`
        (if (`self.LeftCanFlicker`)
          (if (> (- (`KismetSystemLibrary.GetGameTimeInSeconds`) (`self.FlickerLeftLast`) (`self.FlickerLeftInterval`)) 0.0)
            (set `self.LeftCanFlicker` false)
            (set `self.LeftFlickerMaxCount` (* (`KismetMathLibrary.RandomIntegerInRange` 1 5) 2))
            (bind _returnvalue (`KismetSystemLibrary.K2_SetTimerDelegate` (delegate `FlickerLeftEvent`) 0.05 true)))))
      (:`then_1`
        (if (`self.RightCanFlicker`)
          (if (> (- (`KismetSystemLibrary.GetGameTimeInSeconds`) (`self.FlickerRightLast`) (`self.FlickerRightInterval`)) 0.0)
            (set `self.RightCanFlicker` false)
            (set `self.RightFlickerMaxCount` (* (`KismetMathLibrary.RandomIntegerInRange` 1 5) 2))
            (bind _returnvalue_2 (`KismetSystemLibrary.K2_SetTimerDelegate` (delegate `FlickerRightEvent`) 0.05 true))))))))

(event `FlickerLeftEvent`
  (`self.ToggleLight` (`self.LeftLights`))
  ;[1 1 1] Stop flicker timmer after flicker count reached
  (bind _result (`/Engine/EditorBlueprintResources/StandardMacros.IncrementInt` (`self.LeftFlickerCount`))
    (:`  `
      (if (> _result (`self.LeftFlickerMaxCount`))
        (`KismetSystemLibrary.K2_ClearAndInvalidateTimerHandle` (stale `self.ReceiveTick` _returnvalue))
        ;[1 1 1] Reset Flicker vairable
        (set `self.FlickerLeftLast` (`KismetSystemLibrary.GetGameTimeInSeconds`))
        (set `self.LeftCanFlicker` true)
        (set `self.LeftFlickerCount` 0)
        ;[1 1 1] Turn light back on
        (`self.ToggleLight` (`self.LeftLights`))
        (set `self.FlickerLeftInterval` (`self.Get Random Interval Time`))))))

(event `FlickerRightEvent`
  (`self.ToggleLight` (`self.RightLights`))
  ;[1 1 1] Stop flicker timmer after flicker count reached
  (bind _result (`/Engine/EditorBlueprintResources/StandardMacros.IncrementInt` (`self.RightFlickerCount`))
    (:`  `
      (if (> _result (`self.RightFlickerMaxCount`))
        (`KismetSystemLibrary.K2_ClearAndInvalidateTimerHandle` (stale `self.ReceiveTick` _returnvalue_2))
        ;[1 1 1] Reset Flicker vairable
        (set `self.FlickerRightLast` (`KismetSystemLibrary.GetGameTimeInSeconds`))
        (set `self.RightCanFlicker` true)
        (set `self.RightFlickerCount` 0)
        ;[1 1 1] Turn light back on
        (`self.ToggleLight` (`self.RightLights`))
        (set `self.FlickerRightInterval` (`self.Get Random Interval Time`))))))

(fn `FlickerLights`
  (params (Lights :type "Array of LightComponent Object Reference"))
  (for _ (range 2)
    (`self.ToggleLight` Lights)))

(fn `Get Random Interval Time`
  (returns (IntervalTime :type "Float (double-precision)"))
  (return (`KismetMathLibrary.RandomFloatInRange` (`self.LightFlickerMinInterval`) (`self.LightFlickerMaxInterval`))))

(fn `ToggleLight`
  (params (Array :type "Array of LightComponent Object Reference"))
  (for _array_element Array
    (`SceneComponent.ToggleVisibility` _array_element false)))

(fn `UserConstructionScript`)