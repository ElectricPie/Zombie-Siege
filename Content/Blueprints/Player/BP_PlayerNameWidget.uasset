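; BP_PlayerNameWidget is an actor that displays a player's name through a widget component holding a W_PlayerName widget.
; On BeginPlay it caches the cast widget reference.
; SetPlayerName forwards the name to the widget, re-fetching and caching the reference first if it is not yet valid.
; SetWidgetVisablitiy shows or hides the widget component and its children.
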(event `self.ReceiveBeginPlay`
  (bind _asw_player_name (cast `/Game/UI/Widgets/W_PlayerName` (`WidgetComponent.GetWidget` (`self.PlayerNameWidgetComponent`))))
  (set `self.PlayerNameWidget` _asw_player_name))

(fn `SetPlayerName`
  (params (NewName :type String))
  (`self.PlayerNameWidget`
    (:`then`
      _)
    (:`else`
      (bind _asw_player_name (cast `/Game/UI/Widgets/W_PlayerName` (`WidgetComponent.GetWidget` (`self.PlayerNameWidgetComponent`))))
      (set `self.PlayerNameWidget` _asw_player_name)))
  (`/Game/UI/Widgets/W_PlayerName.SetName` (`self.PlayerNameWidget`) (`local.NewName`)))

(fn `SetWidgetVisablitiy`
  (params (IsVisable :type Boolean))
  (`SceneComponent.SetVisibility` (`self.PlayerNameWidgetComponent`) IsVisable true))

(fn `UserConstructionScript`)